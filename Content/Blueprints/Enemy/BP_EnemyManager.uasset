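; Enemy manager that pre-spawns a pool of BP_Enemy actors and releases them on a timer.
; On BeginPlay it initializes each with random Y position and speed, gives TrackerCount of them a separate enemy type, then shuffles the pool.
; Each tick of the looping timer activates the next enemy until the pool is exhausted, with no recycling.
; DeadReport counts down deaths and calls OnFinishedGame at zero, while EndGame stops spawning.
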(event `self.ReceiveBeginPlay`
  (`self.EnemyPooling`)
  (`KismetSystemLibrary.K2_SetTimer` null "SpawnEnemy" (`self.SpawnTimer`) true))

(fn `DeadReport`
  (bind _result (`/Engine/EditorBlueprintResources/StandardMacros.DecrementInt` (`self.EnemyPoolingCount`))
    (:`  `
      (if (<= _result 0)
        (`self.OnFinishedGame`)))))

(fn `EndGame`
  (`KismetSystemLibrary.K2_ClearTimer` null "SpawnEnemy"))

(fn `EnemyPooling`
  (bind (_returnvalue_x _returnvalue_y _returnvalue_z) (`KismetMathLibrary.BreakVector` (`self.K2_GetActorLocation`)))
  (bind (_randomspeedrange_x _randomspeedrange_y) (`KismetMathLibrary.BreakVector2D` (`self.RandomSpeedRange`)))
  (bind _randompositionyrange (`self.RandomPositionYRange`))
  (for _ (range (`self.EnemyPoolingCount`))
    (bind _returnvalue (`|SpawnActorFromClass` "/Game/Blueprints/Enemy/BP_Enemy.BP_Enemy_C" (`KismetMathLibrary.MakeTransform` (`KismetMathLibrary.MakeVector` _returnvalue_x (`KismetMathLibrary.RandomFloatInRange` (* _randompositionyrange -1.0) _randompositionyrange) _returnvalue_z) (struct :`Roll` 180.0)) "AlwaysSpawn" "MultiplyWithRoot" self null))
    (bind _returnvalue_2 (`KismetArrayLibrary.Array_Add` (`self.EnemyPoolStack`) _returnvalue))
    (`/Game/Blueprints/Enemy/BP_Enemy.InitializeEnemy` _returnvalue (`KismetMathLibrary.RandomFloatInRange` _randomspeedrange_x _randomspeedrange_y) (select `bool` (< _returnvalue_2 (`self.TrackerCount`)) :`false` "NewEnumerator0" :`true` "NewEnumerator1" :!type "/Game/Blueprints/Enumeration/E_EnemyType Enum")))
  (`KismetArrayLibrary.Array_Shuffle` (`self.EnemyPoolStack`)))

(fn `SpawnEnemy`
  (`/Game/Blueprints/Enemy/BP_Enemy.SpawnEnemy` (`|GetArrayItem` (`self.EnemyPoolStack`) (`self.PoolIndex`)))
  (bind _result (`/Engine/EditorBlueprintResources/StandardMacros.IncrementInt` (`self.PoolIndex`))
    (:`  `
      (if (>= _result (`KismetArrayLibrary.Array_Length` (`self.EnemyPoolStack`)))
        (`KismetSystemLibrary.K2_ClearTimer` null "SpawnEnemy")))))

(fn `UserConstructionScript`)