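; Enemy actor owned by BP_EnemyManager that starts hidden, is shown on spawn, and hides with an explosion and a manager report on death.
; Base types move straight down, while Trackers home on the player until a height threshold, then descend.
; Trackers smoothly roll toward the player in the YZ plane, using dot and cross products for angle and side.
; Leaving the area triggers delayed death, and killing the player ends the game.
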(event `self.ReceiveBeginPlay`
  (`self.SetHiddenEnemy` true)
  (set `self.TargetRotation` (`self.K2_GetActorRotation`)))

(event `self.ReceiveTick`
  (params (DeltaSeconds :type "Float (single-precision)"))
  (if (not (`self.bHidden`))
    (`self.SearchingPlayer`)
    (`self.TrackingTargetPoint`)))

(event `AreaOut`
  (`KismetSystemLibrary.Delay` 3.0)
  (`self.DeadEnemy`))

(fn `DeadEnemy`
  (`self.SetHiddenEnemy` true)
  (`GameplayStatics.SpawnEmitterAtLocation` "/Game/StarterContent/Particles/P_Explosion.P_Explosion" (`self.K2_GetActorLocation`) (struct) (1.0 1.0 1.0) true "AutoRelease")
  (bind _asbp_enemy_manager (cast `/Game/Blueprints/Enemy/BP_EnemyManager` (`self.GetOwner`)))
  (`/Game/Blueprints/Enemy/BP_EnemyManager.DeadReport` _asbp_enemy_manager))

(fn `GetEnemyScore`
  (returns (score :type Integer))
  (return (`self.EnemyScore`)))

(fn `InitializeEnemy`
  (params (speed :type "Float (double-precision)") (enemyType :type "/Game/Blueprints/Enumeration/E_EnemyType Enum" :default "NewEnumerator0"))
  (set `/Game/Blueprints/Components/BaseMovementComponent.MoveSpeed` speed (`self.BaseMovementComponent`))
  (bind _output_get (set `self.ThisEnemyType` enemyType))
  (set `self.EnemyScore` (select `/Game/Blueprints/Enumeration/E_EnemyType` _output_get :`NewEnumerator0` 10 :`NewEnumerator1` 30)))

(fn `PlayerKill`
  (bind _asbp_enemy_manager (cast `/Game/Blueprints/Enemy/BP_EnemyManager` (`self.GetOwner`)))
  (`/Game/Blueprints/Enemy/BP_EnemyManager.EndGame` _asbp_enemy_manager))

(fn `SearchingPlayer`
  (bind _returnvalue (`self.GetActorUpVector`))
  (bind _output_get (set `self.PlayerTargetPosition` (`self.K2_GetActorLocation` (`GameplayStatics.GetPlayerPawn` 0))))
  (bind _returnvalue_2 (`KismetMathLibrary.Normal` (`KismetMathLibrary.MakeVector` 0.0 (.y (- _output_get (`self.K2_GetActorLocation`))) (.z (- _output_get (`self.K2_GetActorLocation`))))))
  (bind _returnvalue_3 (`KismetMathLibrary.DegAcos` (`KismetMathLibrary.Dot_VectorVector` _returnvalue _returnvalue_2)))
  ;[0 0 1] X축 역방향을 상단으로 기준으로 하야 해당 각도만큼 이동시킨 회전값 저장
  (set `self.TargetRotation` (`KismetMathLibrary.RotatorFromAxisAndAngle` (-1.0 0.0 0.0) (+ (.roll (`self.K2_GetActorRotation`)) (select `bool` (> (.x (`KismetMathLibrary.Cross_VectorVector` _returnvalue _returnvalue_2)) 0.0) :`false` _returnvalue_3 :`true` (* _returnvalue_3 -1.0))))))

(fn `SetHiddenEnemy`
  (params (hidden :type Boolean))
  (`self.SetActorHiddenInGame` hidden)
  (`PrimitiveComponent.SetCollisionEnabled` (`self.Sphere`) (select `bool` hidden :`false` "QueryAndPhysics" :`true` "NoCollision" :!type "ECollisionEnabled Enum")))

(fn `SpawnEnemy`
  (`self.SetHiddenEnemy` false))

(fn `TrackingTargetPoint`
  (bind (_returnvalue_x _returnvalue_y _returnvalue_z) (`KismetMathLibrary.BreakVector` (`self.K2_GetActorLocation`)))
  (bind _basemovementcomponent (`self.BaseMovementComponent`))
  (bind _returnvalue (> _returnvalue_z -250.0))
  (bind _asbp_my_player_pawn (cast `/Game/Blueprints/Player/BP_MyPlayerPawn` (`GameplayStatics.GetPlayerPawn` 0)))
  (if (`/Game/Blueprints/Player/BP_MyPlayerPawn.IsPlayerDead?` _asbp_my_player_pawn)
    (`/Game/Blueprints/Components/BaseMovementComponent.SetMovementDirection` _basemovementcomponent (0.0 0.0 0.0))
    (elif (`|EnumEquality` (`self.ThisEnemyType`) "NewEnumerator0")
      (`/Game/Blueprints/Components/BaseMovementComponent.SetMovementDirection` _basemovementcomponent (0.0 0.0 -1.0))
      (else
        (`/Game/Blueprints/Components/BaseMovementComponent.SetMovementDirection` _basemovementcomponent (select `bool` _returnvalue :`false` (0.0 0.0 -1.0) :`true` (`KismetMathLibrary.Normal` (- (`self.PlayerTargetPosition`) (`self.K2_GetActorLocation`)))))
        (if (not _returnvalue)
          (set `self.TargetRotation` (struct :`Roll` 180.0)))
        (`self.K2_SetActorRotation` (`KismetMathLibrary.RInterpTo` (`self.K2_GetActorRotation`) (`self.TargetRotation`) (`GameplayStatics.GetWorldDeltaSeconds`) (`self.RotateInterpSpeed`)))))))

(fn `UserConstructionScript`)