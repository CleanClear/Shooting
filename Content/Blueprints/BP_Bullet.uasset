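; BP_Bullet is a reusable projectile that kills enemies and awards score to its owning BP_MyPlayerPawn.
; It starts hidden without collision; FireBullet teleports it into place, sets its movement direction, shows it and starts a hide timer.
; Overlapping a BP_Enemy kills it, plays an explosion cue, hides the bullet, updates the score and clears the timer.
; The actor is toggled rather than destroyed, with IsFire tracking whether it is in flight.
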(event `self.ReceiveBeginPlay`
  (`self.SetVisibilityBullet` false))

(event `self.Cube.OnComponentBeginOverlap`
  (params (OverlappedComponent :type "PrimitiveComponent Object Reference") (OtherActor :type "Actor Object Reference") (OtherComp :type "PrimitiveComponent Object Reference") (OtherBodyIndex :type Integer) (bFromSweep :type Boolean) (SweepResult :type "HitResult Structure (by ref)"))
  ;[0 0 0] 총알이 적을 맞췄을 때 판정
  (bind _asbp_enemy (cast `/Game/Blueprints/Enemy/BP_Enemy` OtherActor))
  (`/Game/Blueprints/Enemy/BP_Enemy.DeadEnemy` _asbp_enemy)
  (`self.PlayAudioToSound` "/Game/Audio/Cue_BoomEnemy.Cue_BoomEnemy")
  (set `self.IsFire` false)
  (`self.SetVisibilityBullet` false)
  (bind _asbp_my_player_pawn (cast `/Game/Blueprints/Player/BP_MyPlayerPawn` (`self.GetOwner`)))
  (`/Game/Blueprints/Player/BP_MyPlayerPawn.UpdateScore` _asbp_my_player_pawn (`/Game/Blueprints/Enemy/BP_Enemy.GetEnemyScore` _asbp_enemy))
  (`KismetSystemLibrary.K2_ClearTimer` null "HiddenBullet"))

(fn `FireBullet`
  (params (firePosition :type "Vector Structure") (direction :type "Vector Structure"))
  (if (`self.IsFire`)
    (`KismetSystemLibrary.K2_ClearTimer` null "HiddenBullet")
    (else
      (set `self.IsFire` true)))
  (`self.K2_SetActorLocation` firePosition false true)
  (`/Game/Blueprints/Components/BaseMovementComponent.SetMovementDirection` (`self.BaseMovementComponent`) direction)
  (`self.SetVisibilityBullet` true)
  (`KismetSystemLibrary.K2_SetTimer` null "HiddenBullet" (`self.BulletHiddenTime`)))

(fn `HiddenBullet`
  (`self.SetVisibilityBullet` false)
  (set `self.IsFire` false))

(fn `PlayAudioToSound`
  (params (NewSound :type "SoundBase Object Reference"))
  (bind _audio (`self.Audio`))
  (`AudioComponent.SetSound` _audio NewSound)
  (`AudioComponent.Play` _audio 0.0))

(fn `SetVisibilityBullet`
  (params (visibility :type Boolean))
  (`self.SetActorHiddenInGame` (not visibility))
  (`PrimitiveComponent.SetCollisionEnabled` (`self.Cube`) (select `bool` visibility :`false` "NoCollision" :`true` "QueryOnly" :!type "ECollisionEnabled Enum")))

(fn `UserConstructionScript`)