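; Base movement component that moves its owning actor at a set velocity.
; SetMovementDirection sets Velocity to the given direction scaled by MoveSpeed.
; Each Tick, UpdateMovement offsets the owner in world space by Velocity times delta time, with UseBlockingCollision deciding whether the move sweeps for collision.
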(event `self.ReceiveBeginPlay`)

(event `self.ReceiveTick`
  (params (DeltaSeconds :type "Float (single-precision)"))
  (`self.UpdateMovement` DeltaSeconds))

(fn `SetMovementDirection`
  (params (direction :type "Vector Structure"))
  (set `self.Velocity` (* direction (`self.MoveSpeed`))))

(fn `UpdateMovement`
  (params (deltaTime :type "Float (double-precision)"))
  (`Actor.K2_AddActorWorldOffset` (`self.GetOwner`) (* deltaTime (`self.Velocity`)) (`self.UseBlockingCollision`) false))