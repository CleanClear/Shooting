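; Player pawn Blueprint that manages a WB_AreaTest score widget on screen.
; ShowWidget lazily creates and caches the widget, then adds it to the viewport and sets a shown flag that guards repeat adds.
; CloseWidget removes the widget when that flag is set but never clears it, so ShowWidget does not re-add a still-valid widget.
; The UpdateScore event writes the score directly into the cached widget without a validity check.
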(event `self.ReceiveBeginPlay`)

(event `self.ReceiveUpdateScore`
  (params (score :type Integer))
  (set `/Game/Blueprints/WB_AreaTest.Score` score (`self.ScreeWidget`)))

(fn `CloseWidget`
  (if (`self.WidgetIsShow`)
    (`Widget.RemoveFromParent` (`self.ScreeWidget`))))

(fn `ShowWidget`
  (`self.ScreeWidget`
    (:`then`
      (if (not (`self.WidgetIsShow`))
        (`UserWidget.AddToViewport` (stale _output_get) 0 :!label _label)
        (set `self.WidgetIsShow` true)))
    (:`else`
      (bind _returnvalue (`|CreateWidget` "/Game/Blueprints/WB_AreaTest.WB_AreaTest_C"))
      (bind _output_get (set `self.ScreeWidget` _returnvalue))
      (goto _label))))

(fn `UserConstructionScript`)