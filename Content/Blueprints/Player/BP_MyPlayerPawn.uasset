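; Player spaceship pawn for a shooter, with axis movement, boost, firing, score tracking and death on enemy collision.
; Movement input feeds BaseMovementComponent and an interpolated horizontal tilt, with boost doubling both speeds.
; BeginPlay pre-spawns a bullet pool that FireAction cycles round-robin, in single shots or a Gate/Delay auto-fire loop.
; Enemy hits explode and hide the ship, while BP_EnemyManager's finish event prints the clear score.
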(event `self.ReceiveTick`
  (params (DeltaSeconds :type "Float (single-precision)"))
  (if (not (`self.IsDead`))
    (`self.UpdateTiltingFlight` DeltaSeconds)))

(event `self.ReceiveBeginPlay`
  ;[0 0 0] 초기화
  (`KismetSystemLibrary.PrintString` "Hello world!")
  (`self.LockAndLoad`)
  (bind _returnvalue (`GameplayStatics.GetActorOfClass` "/Game/Blueprints/Enemy/BP_EnemyManager.BP_EnemyManager_C"))
  (bind _output_get (set `self.EnemyManager` _returnvalue))
  (add `/Game/Blueprints/Enemy/BP_EnemyManager.OnFinishedGame` _output_get (delegate `OnFinishedGame_이벤트`)))

(event `OnFinishedGame_이벤트`
  ;[0 0 0] 초기화
  (`KismetSystemLibrary.PrintString` (`KismetStringLibrary.Concat_StrStr` "Game Clear (Total Score : " (`KismetStringLibrary.Conv_IntToString` (`self.TotalScore`)) ")")))

(event `InputAction|Fire`
  (params (Key :type "Key Structure"))
  ;[0 0 0] 사격 Input Action : 연사 / 단발
  (:`Pressed`
    (if (`self.IsDead`)
      _
      (elif (`self.AutoFireMode`)
        (`self.FireToDelay`)
        (else
          (`self.FireAction`)))))
  (:`Released`
    (set `self.IsFiring` false)))

(event `InputAxis|Horizontal`
  (params (AxisValue :type "Float (single-precision)"))
  (bind (_currentmovedirection_x _currentmovedirection_y _currentmovedirection_z) (`KismetMathLibrary.BreakVector` (`self.CurrentMoveDirection`)))
  ;[0 0 0] 이동 관련 Input Key Event
  (if (not (`self.IsDead`))
    (bind _output_get (set `self.CurrentMoveDirection` (`KismetMathLibrary.MakeVector` _currentmovedirection_x AxisValue _currentmovedirection_z)))
    (`/Game/Blueprints/Components/BaseMovementComponent.SetMovementDirection` (`self.BaseMovementComponent`) _output_get)
    (`self.SetHorizontalTiltTarget` AxisValue)))

(event `FireToDelay`
  ;[0 0 0] 연사 모드
  (`self.FireAction`)
  (`|ExecutionSequence`
    (:`then_0`
      (goto _label :!via `Open`))
    (:`then_1`
      (`/Engine/EditorBlueprintResources/StandardMacros.Gate` true :!label _label
        (:`Exit`
          (`KismetSystemLibrary.Delay` (`self.FireDelay`))
          (if (`self.IsFiring`)
            (`self.FireAction`)
            (goto _label)
            (else
              (goto _label :!via `Close`))))))))

(event `InputAxis|Vertical`
  (params (AxisValue :type "Float (single-precision)"))
  (bind (_currentmovedirection_x _currentmovedirection_y) (`KismetMathLibrary.BreakVector` (`self.CurrentMoveDirection`)))
  ;[0 0 0] 이동 관련 Input Key Event
  (if (not (`self.IsDead`))
    (bind _output_get (set `self.CurrentMoveDirection` (`KismetMathLibrary.MakeVector` _currentmovedirection_x _currentmovedirection_y AxisValue)))
    (`/Game/Blueprints/Components/BaseMovementComponent.SetMovementDirection` (`self.BaseMovementComponent`) _output_get)))

(event `self.Sphere.OnComponentHit`
  (params (HitComponent :type "PrimitiveComponent Object Reference") (OtherActor :type "Actor Object Reference") (OtherComp :type "PrimitiveComponent Object Reference") (NormalImpulse :type "Vector Structure") (Hit :type "HitResult Structure (by ref)"))
  ;[0 0 0] 게임 오버
  (bind _asbp_enemy (cast `/Game/Blueprints/Enemy/BP_Enemy` OtherActor))
  (`/Game/Blueprints/Enemy/BP_Enemy.PlayerKill` _asbp_enemy)
  (set `self.IsDead` true)
  (set `self.CurrentMoveDirection` (0.0 0.0 0.0))
  (set `self.IsFiring` false)
  (`GameplayStatics.SpawnEmitterAtLocation` "/Game/StarterContent/Particles/P_Explosion.P_Explosion" (`self.K2_GetActorLocation`) (struct) (1.0 1.0 1.0) true "AutoRelease")
  (`self.PlayAudioToSound` "/Game/StarterContent/Audio/Cue_PlayerBoom.Cue_PlayerBoom")
  (`self.SetActorHiddenInGame` true)
  (`PrimitiveComponent.SetCollisionEnabled` (`self.Sphere`) "NoCollision")
  (`KismetSystemLibrary.PrintString` "Game Over!"))

(event `InputAction|boost`
  (params (Key :type "Key Structure"))
  (bind _basemovementcomponent (`self.BaseMovementComponent`))
  (bind _movespeed (`/Game/Blueprints/Components/BaseMovementComponent.MoveSpeed` _basemovementcomponent))
  ;[0 0 0] 이동 관련 Input Key Event
  (:`Pressed`
    (set `/Game/Blueprints/Components/BaseMovementComponent.MoveSpeed` (* _movespeed 2.0) _basemovementcomponent)
    (set `self.IsBoost` true))
  (:`Released`
    (set `/Game/Blueprints/Components/BaseMovementComponent.MoveSpeed` (* _movespeed 0.5) _basemovementcomponent)
    (set `self.IsBoost` false)))

(fn `FireAction`
  (set `self.IsFiring` true)
  (bind _asbp_bullet (cast `/Game/Blueprints/BP_Bullet` (`|GetArrayItem` (`self.BulletMagazine`) (`self.PoolBulletIndex`))))
  (`/Game/Blueprints/BP_Bullet.FireBullet` _asbp_bullet (`SceneComponent.K2_GetComponentLocation` (`self.SpaceShip`)) (`self.GetActorUpVector`))
  (set `self.PoolBulletIndex` (mod (+ (`self.PoolBulletIndex`) 1) (`self.MaxMagazineBullets`)))
  (`GameplayStatics.SpawnSound2D` "/Game/Audio/Cue_FireSound.Cue_FireSound" 1.0 1.0 0.0 null))

(fn `IsPlayerDead?`
  (returns (playerDead :type Boolean))
  (return (`self.IsDead`)))

(fn `LockAndLoad`
  (for _ (range (`self.MaxMagazineBullets`))
    (bind _returnvalue (`|SpawnActorFromClass` "/Game/Blueprints/BP_Bullet.BP_Bullet_C" (`KismetMathLibrary.MakeTransform` (0.0 0.0 0.0)) "AlwaysSpawn" "MultiplyWithRoot" self null))
    (`KismetArrayLibrary.Array_Add` (`self.BulletMagazine`) _returnvalue)))

(fn `PlayAudioToSound`
  (params (NewSound :type "SoundBase Object Reference"))
  (bind _playeraudio (`self.PlayerAudio`))
  (`AudioComponent.SetSound` _playeraudio NewSound)
  (`AudioComponent.Play` _playeraudio 0.0))

(fn `SetHorizontalTiltTarget`
  (params (axis :type "Float (double-precision)"))
  (bind _horizontaltiltrotdegrees (`self.HorizontalTiltRotDegrees`))
  (set `self.TargetTiltRotDegrees` (`KismetMathLibrary.MapRangeClamped` axis -1.0 1.0 _horizontaltiltrotdegrees (* _horizontaltiltrotdegrees -1.0))))

(fn `UpdateScore`
  (params (Score :type Integer))
  (set `self.TotalScore` (+ Score (`self.TotalScore`))))

(fn `UpdateTiltingFlight`
  (params (deltaTime :type "Float (double-precision)"))
  (bind _tiltinginterpspeed (`self.TiltingInterpSpeed`))
  (bind (_relativerotation_roll _relativerotation_pitch _relativerotation_yaw) (`KismetMathLibrary.BreakRotator` (`SceneComponent.RelativeRotation` (`self.Scene`))))
  (`SceneComponent.K2_SetRelativeRotation` (`self.Scene`) (`KismetMathLibrary.MakeRotator` 0.0 0.0 (`KismetMathLibrary.FInterpTo` _relativerotation_yaw (`self.TargetTiltRotDegrees`) deltaTime (select `bool` (`self.IsBoost`) :`false` _tiltinginterpspeed :`true` (* _tiltinginterpspeed 2.0)))) false false))

(fn `UserConstructionScript`)